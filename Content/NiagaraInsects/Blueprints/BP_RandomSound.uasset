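; Actor that plays a randomized, continuous insect ambience at its location.
; After a spawn delay on BeginPlay, it starts six parallel sound voices, two for each of its three sounds.
; Each voice plays with random volume and pitch through insect attenuation, then binds its audio-finished event back to itself, so it repeats endlessly with fresh variation.
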(event `self.ReceiveBeginPlay`
  (`KismetSystemLibrary.Delay` (`self.SpawnDelay`))
  (`self.StartSounds_1`)
  (`self.StartSounds_2`)
  (`self.StartSounds_3`)
  (`self.StartSounds_4`)
  (`self.StartSounds_5`)
  (`self.StartSounds_6`))

(event `StartSounds_1`
  (bind _returnvalue (`GameplayStatics.SpawnSoundAtLocation` (`self.Sound_1`) (`self.K2_GetActorLocation`) (struct) (`KismetMathLibrary.RandomFloatInRange` 0.0 1.0) (`KismetMathLibrary.RandomFloatInRange` 1.0 3.0) 0.0 "/Game/NiagaraInsects/Sounds/SA_Insects.SA_Insects" null))
  (add `AudioComponent.OnAudioFinished` _returnvalue (delegate `StartSounds_1`)))

(event `StartSounds_4`
  (bind _returnvalue (`GameplayStatics.SpawnSoundAtLocation` (`self.Sound_1`) (`self.K2_GetActorLocation`) (struct) (`KismetMathLibrary.RandomFloatInRange` 0.0 1.0) (`KismetMathLibrary.RandomFloatInRange` 1.0 3.0) 0.0 "/Game/NiagaraInsects/Sounds/SA_Insects.SA_Insects" null))
  (add `AudioComponent.OnAudioFinished` _returnvalue (delegate `StartSounds_4`)))

(event `StartSounds_2`
  (bind _returnvalue (`GameplayStatics.SpawnSoundAtLocation` (`self.Sound_2`) (`self.K2_GetActorLocation`) (struct) (`KismetMathLibrary.RandomFloatInRange` 0.0 1.0) (`KismetMathLibrary.RandomFloatInRange` 1.0 3.0) 0.0 "/Game/NiagaraInsects/Sounds/SA_Insects.SA_Insects" null))
  (add `AudioComponent.OnAudioFinished` _returnvalue (delegate `StartSounds_2`)))

(event `StartSounds_5`
  (bind _returnvalue (`GameplayStatics.SpawnSoundAtLocation` (`self.Sound_2`) (`self.K2_GetActorLocation`) (struct) (`KismetMathLibrary.RandomFloatInRange` 0.0 1.0) (`KismetMathLibrary.RandomFloatInRange` 1.0 3.0) 0.0 "/Game/NiagaraInsects/Sounds/SA_Insects.SA_Insects" null))
  (add `AudioComponent.OnAudioFinished` _returnvalue (delegate `StartSounds_5`)))

(event `StartSounds_3`
  (bind _returnvalue (`GameplayStatics.SpawnSoundAtLocation` (`self.Sound_3`) (`self.K2_GetActorLocation`) (struct) (`KismetMathLibrary.RandomFloatInRange` 0.0 1.0) (`KismetMathLibrary.RandomFloatInRange` 1.0 3.0) 0.0 "/Game/NiagaraInsects/Sounds/SA_Insects.SA_Insects" null))
  (add `AudioComponent.OnAudioFinished` _returnvalue (delegate `StartSounds_3`)))

(event `StartSounds_6`
  (bind _returnvalue (`GameplayStatics.SpawnSoundAtLocation` (`self.Sound_3`) (`self.K2_GetActorLocation`) (struct) (`KismetMathLibrary.RandomFloatInRange` 0.0 1.0) (`KismetMathLibrary.RandomFloatInRange` 1.0 3.0) 0.0 "/Game/NiagaraInsects/Sounds/SA_Insects.SA_Insects" null))
  (add `AudioComponent.OnAudioFinished` _returnvalue (delegate `StartSounds_6`)))

(fn `UserConstructionScript`)