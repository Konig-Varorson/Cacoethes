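; Base weapon Blueprint for the first-person player, handling hitscan firing, ammo and reload.
; WeaponFire spends a round and calls CalculateShot, a debug-drawn camera line trace with random endpoint spread; muzzle socket inputs don't affect it.
; Only Ue4ASP_Character hits trigger mesh physics, a zero impulse and an impact effect.
; Reload refills from reserve, discarding remaining rounds; ammo query helpers exist, but WeaponFire doesn't check them.
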(event `self.ReceiveBeginPlay`
  (bind _asfirst_person_character (cast `/Game/Blueprints/FirstPersonCharacter` (`GameplayStatics.GetPlayerPawn` 0)))
  (set `self.PlayerREF` _asfirst_person_character))

(fn `CalculateShot`
  (params (Camera :type "CameraComponent Object Reference") (WeaponMesh :type "SceneComponent Object Reference") (WeaponFireSocketName :type Name))
  (returns (HitResult :type "HitResult Structure"))
  (locals (LocalCamera :type "CameraComponent Object Reference") (LocalWeaponMesh :type "SceneComponent Object Reference") (LocalSocketName :type Name))
  (bind _bulletspread (`self.BulletSpread`))
  (bind (_returnvalue_location _returnvalue_rotation) (`KismetMathLibrary.BreakTransform` (`SceneComponent.K2_GetComponentToWorld` (`local.LocalCamera`))))
  (bind _returnvalue (* _bulletspread -1.0))
  (`|ExecutionSequence`
    (:`then_0`
      (set `local.LocalCamera` Camera)
      (set `local.LocalWeaponMesh` WeaponMesh)
      (set `local.LocalSocketName` WeaponFireSocketName))
    (:`then_1`
      (bind _outhit (`KismetSystemLibrary.LineTraceSingleForObjects` _returnvalue_location (`KismetMathLibrary.MakeVector` (+ (.x (+ _returnvalue_location (* (`KismetMathLibrary.GetForwardVector` _returnvalue_rotation) (`self.BulletDistance`)))) (`KismetMathLibrary.RandomFloatInRange` _returnvalue _bulletspread)) (+ (.y (+ _returnvalue_location (* (`KismetMathLibrary.GetForwardVector` _returnvalue_rotation) (`self.BulletDistance`)))) (`KismetMathLibrary.RandomFloatInRange` _returnvalue _bulletspread)) (+ (.z (+ _returnvalue_location (* (`KismetMathLibrary.GetForwardVector` _returnvalue_rotation) (`self.BulletDistance`)))) (`KismetMathLibrary.RandomFloatInRange` _returnvalue _bulletspread))) (`|MakeArray` "ObjectTypeQuery1" "ObjectTypeQuery2" "ObjectTypeQuery4" :!type "EObjectTypeQuery Enum") false (`|MakeArray` (`GameplayStatics.GetPlayerPawn` 0) :!type "Actor Object Reference") "ForDuration"))
      (return _outhit))))

(fn `HasAmmoInMag`
  (returns (HasAmmo :type Boolean) (MagFull :type Boolean))
  (bind _currentammo (`self.CurrentAmmo`))
  (return (> _currentammo 0) (== _currentammo (`self.MaxAmmo`))))

(fn `HasExtraAmmo`
  (returns (HasExtraAmmo :type Boolean))
  (return (> (`self.CurrentTotalAmmo`) 0)))

(fn `UserConstructionScript`)

(fn `WeaponFire`
  (if true
    (set `self.CurrentAmmo` (- (`self.CurrentAmmo`) 1))
    (bind _hitresult (`self.CalculateShot` (`/Game/Blueprints/FirstPersonCharacter.FirstPersonCamera` (`self.PlayerREF`)) null "MuzzleFlash"))
    (bind (_bblockinghit _binitialoverlap _time _distance _location _impactpoint _normal _impactnormal _physmat _hitactor _hitcomponent _hitbonename) (`GameplayStatics.BreakHitResult` _hitresult))
    (bind _asue_4asp_character (cast `/Game/AnimStarterPack/Ue4ASP_Character` _hitactor))
    (bind _mesh (`Character.Mesh` _asue_4asp_character))
    (`PrimitiveComponent.SetSimulatePhysics` _mesh true)
    (`PrimitiveComponent.AddImpulse` _mesh (0.0 0.0 0.0) _hitbonename true)
    (`|SpawnActorFromClass` (`self.ImpactEffectClass`) (`KismetMathLibrary.MakeTransform` _impactpoint) "Undefined" "OverrideRootScale" null _hitresult _bblockinghit null)
    (return)))

(fn `WeaponReload`
  (bind _returnvalue (`KismetMathLibrary.Min` (`self.MaxAmmo`) (`self.CurrentTotalAmmo`)))
  (set `self.CurrentAmmo` _returnvalue)
  (set `self.CurrentTotalAmmo` (- (`self.CurrentTotalAmmo`) _returnvalue)))